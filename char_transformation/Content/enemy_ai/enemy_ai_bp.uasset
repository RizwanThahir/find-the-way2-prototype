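; Enemy AI Blueprint that chases the player and throws a punch once it gets close.
; PawnSensing's see-pawn event sets a seeing flag and calls the follow event, which uses AI MoveTo toward player pawn 0.
; On a successful move it plays the punch montage, gating repeat attacks with a flag and a delay equal to the montage length.
; The seeing flag is never cleared within this graph.
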(event `self.PawnSensing.OnSeePawn`
  (params (Pawn :type "Pawn Object Reference"))
  (set `self.is_seeing?` true)
  (`self.fellowplayer`))

(event `fellowplayer`
  (set `self.can_attack?` true)
  (if (`self.is_seeing?`)
    (`|AIMoveTo` self (0.0 0.0 0.0) (`GameplayStatics.GetPlayerPawn` 0) 70.0
      (:`OnSuccess`
        (if (`self.can_attack?`)
          (set `self.can_attack?` false)
          (bind _returnvalue (`self.PlayAnimMontage` "/Game/enemy_ai/anim/enemy_punch_montage.enemy_punch_montage"))
          (`KismetSystemLibrary.Delay` _returnvalue)
          (set `self.can_attack?` true))))))

(fn `UserConstructionScript`)